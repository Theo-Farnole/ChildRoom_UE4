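; Example interactable actor that shows interact text and an outline on its Cube while hovered.
; StartHover calls ShowInteractText, then adds a static mesh component at runtime and passes it with the Cube to ShowOutline.
; EndHover hides the text through the HUD_ThirdPerson actor, destroys the outline component and prints a debug string.
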(event EventEndHover
  (params (hoverActor :type Actor%20Object%20Reference))
  (bind _outlinemesh (Variables|Default|GetOutlineMesh))
  (Utilities|FlowControl|Sequence
    (:then_0
      (bind _returnvalue (Actor|GetActorOfClass "/Game/_BP/_Gamemodes/HUD_ThirdPerson.HUD_ThirdPerson_C"))
      (Default|HideInteractText _returnvalue))
    (:then_1
      (Utilities|IsValid _outlinemesh
        (:Is%20Valid
          (Components|DestroyComponent _outlinemesh))))
    (:then_2
      (Development|PrintString "Hello"))))

(event EventStartHover
  (params (hoverActor :type Actor%20Object%20Reference))
  (Utilities|FlowControl|Sequence
    (:then_0
      (Utilities|ShowInteractText))
    (:then_1
      (bind _returnvalue (AddComponent|AddStaticMeshComponent false))
      (bind _output_get (Variables|Default|SetOutlineMesh _returnvalue))
      (Utilities|ShowOutline (Variables|Default|GetCube) _output_get "(R=0.308644,G=1.000000,B=0.318043,A=1.000000)" 1.0))))

(fn ConstructionScript)