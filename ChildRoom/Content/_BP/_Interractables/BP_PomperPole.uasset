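; BP_PomperPole is an interactable vertical pole that puts a third-person character into a dedicated pole state.
; On Interact it switches the CH_ThirdPerson state and passes itself to the resulting BP_State_PomperPole, printing a bug message if that cast fails.
; It exposes its bottom and top positions, running from the actor location up by PoleLength along world Z.
; The construction script draws that span as a temporary debug line, flushing earlier persistent lines first.
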(event EventInteract
  (params (interactor :type Actor%20Object%20Reference))
  (bind _asch_third_person (Utilities|Casting|CastToCH_ThirdPerson interactor))
  (bind _newstate (Default|SetState _asch_third_person "NewEnumerator3"))
  (bind _asbp_state_pomper_pole (Utilities|Casting|CastToBP_State_PomperPole _newstate)
    (:then
      (Default|SetPomperPole _asbp_state_pomper_pole self))
    (:CastFailed
      (Development|PrintString "This is a bug!"))))

(fn ConstructionScript
  (bind _returnvalue (Transformation|GetActorLocation))
  (Rendering|Debug|FlushPersistentDebugLines)
  (Rendering|Debug|DrawDebugLine _returnvalue (+ _returnvalue (Math|Vector|MakeVector 0.0 0.0 (Variables|Default|GetpoleLength))) "(R=0.418453,G=0.073804,B=0.953125,A=1.000000)" 1e+01 5.0))

(fn GetMaxPosition
  (bind _minposition (CallFunction|GetMinPosition))
  (return (+ _minposition (Math|Vector|MakeVector 0.0 0.0 (Variables|Default|GetpoleLength)))))

(fn GetMinPosition
  (return (Transformation|GetActorLocation self)))

(fn GetBoundsPosition
  (bind _maxposition (CallFunction|GetMaxPosition))
  (bind _minposition (CallFunction|GetMinPosition))
  (return _minposition _maxposition))