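; Base interactable for an object the player can push along an assigned spline rail.
; On BeginPlay it finds its distance along the rail and anchors there, optionally snapping to the ground.
; Interacting switches the player character into a move-object state bound to this actor.
; Push projects a force onto the spline direction to update that distance and draws debug lines, while hovering shows an outline through a temporary mesh component.
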(event EventBeginPlay
  (Utilities|CalculateCurrentPositiononRail)
  (Utilities|AnchoronRail))

(event EventTick
  (params (DeltaSeconds :type Float%20%28single-precision%29))
  (Utilities|FlowControl|Sequence))

(event EventInteract
  (params (interactor :type Actor%20Object%20Reference))
  (bind _asch_third_person (Utilities|Casting|CastToCH_ThirdPerson interactor))
  (bind _newstate (Default|SetState _asch_third_person "NewEnumerator2"))
  (bind _asbp_state_move_object (Utilities|Casting|CastToBP_State_MoveObject _newstate)
    (:then
      (Default|SetMovableObject _asbp_state_move_object self))
    (:CastFailed
      (Development|PrintString "wtf problem in  set state"))))

(event EventEndHover
  (params (hoverActor :type Actor%20Object%20Reference))
  (bind _outlinemesh (Variables|Default|GetOutlineMesh))
  (Utilities|IsValid _outlinemesh
    (:Is%20Valid
      (Components|DestroyComponent _outlinemesh))))

(event EventStartHover
  (params (hoverActor :type Actor%20Object%20Reference))
  (bind _returnvalue (Actor|GetComponentsByClass "/Script/Engine.StaticMeshComponent"))
  (bind _returnvalue_2 (AddComponent|AddStaticMeshComponent false))
  (bind _output_get (Variables|Default|SetOutlineMesh _returnvalue_2))
  (if (> (Utilities|Array|Length _returnvalue) 0)
    (Utilities|ShowOutline (Utilities|Array|Get(acopy) _returnvalue) _output_get "(R=1.000000,G=0.101376,B=0.061575,A=1.000000)" 1.0)
    (else
      (Development|PrintString "Cannot outline MovableObject: no component on this actor."))))

(fn ConstructionScript)

(fn Push
  (params (force :type Vector))
  (bind _returnvalue (Transformation|GetActorLocation))
  (bind _returnvalue_2 (+ _returnvalue "0, 0,30.000000"))
  (Utilities|FlowControl|Sequence
    (:then_0
      (Variables|Default|SetcurrentPositionOnRail (+ (Variables|Default|GetcurrentPositionOnRail) (Math|Vector|DotProduct force (Spline|GetDirectionatDistanceAlongSpline (Variables|/Game/_BP/_Interractables/BP_Rail.BP_Rail_C|GetSpline (Variables|Default|GetRail)) (Variables|Default|GetcurrentPositionOnRail) "World"))))
      (Utilities|AnchoronRail))
    (:then_1
      (Rendering|Debug|DrawDebugLine _returnvalue_2 (+ _returnvalue_2 (* (Spline|GetDirectionatDistanceAlongSpline (Variables|/Game/_BP/_Interractables/BP_Rail.BP_Rail_C|GetSpline (Variables|Default|GetRail)) (Variables|Default|GetcurrentPositionOnRail) "World") (* (Math|Vector|DotProduct force (Spline|GetDirectionatDistanceAlongSpline (Variables|/Game/_BP/_Interractables/BP_Rail.BP_Rail_C|GetSpline (Variables|Default|GetRail)) (Variables|Default|GetcurrentPositionOnRail) "World")) 1e+01))) "(R=0.000000,G=1.000000,B=0.130546,A=1.000000)" 0.0 1.0))
    (:then_2
      (Rendering|Debug|DrawDebugLine _returnvalue_2 (+ _returnvalue_2 (* force 1e+01)) "(R=0.973958,G=0.000000,B=0.133960,A=1.000000)" 0.0 1.0))))