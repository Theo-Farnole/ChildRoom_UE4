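; Interactable button Blueprint that forwards a player's interaction to a linked ActorToInteract through BPI_Interactable.
; When UsableOnce is set, it fires only until the first successful forward, tracked by UsedCount, and prints an error if the target lacks the interface.
; Hovering shows interact text and an outline on a temporary static mesh component copied from the Cube, which is destroyed when hover ends.
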(event EventStartHover
  (params (hoverActor :type Actor%20Object%20Reference))
  (Utilities|FlowControl|Sequence
    (:then_0
      (Utilities|ShowInteractText))
    (:then_1
      (bind _returnvalue (AddComponent|AddStaticMeshComponent false (Math|Transform|MakeTransform "0, 0, 0")))
      (bind _output_get (Variables|Default|SetoutlineSMComponent _returnvalue))
      (Utilities|ShowOutline (Variables|Default|GetCube) _output_get "(R=0.308644,G=1.000000,B=0.318043,A=1.000000)" 1.0))))

(event EventEndHover
  (params (hoverActor :type Actor%20Object%20Reference))
  (Utilities|FlowControl|Sequence
    (:then_0
      (Utilities|HideInteractText))
    (:then_1
      (Components|DestroyComponent (Variables|Default|GetoutlineSMComponent)))))

(event EventInteract
  (params (interactor :type Actor%20Object%20Reference))
  (if (Variables|Default|GetusableOnce)
    (if (== (Variables|Default|GetusedCount) 0)
      (bind _asbpi_interactable (Utilities|Casting|CastToBPI_Interactable (Variables|Default|GetactorToInteract) :!label _label)
        (:then
          (Default|Interact _asbpi_interactable interactor)
          (Math|Integer|IncrementInt (Variables|Default|GetusedCount)))
        (:CastFailed
          (Development|PrintString "Missing BPI Interactable in actor to interact."))))
    (else
      (goto _label))))

(fn ConstructionScript)