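; BP_Bumper is an interactable that launches the third-person character upward when it overlaps the actor.
; On overlap, Bump adds an impulse from GetImpulse to the character's movement component as a velocity change.
; GetImpulse holds the kinematic formula deriving vertical speed from gravity and JumpHeight.
; The construction script draws a debug line previewing JumpHeight above the bumper.
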(event Collision|EventActorBeginOverlap
  (params (OtherActor :type Actor%20Object%20Reference))
  (bind _asch_third_person (Utilities|Casting|CastToCH_ThirdPerson OtherActor))
  (Utilities|Bump (Variables|/Script/Engine.Character|GetCharacterMovement _asch_third_person)))

(fn ConstructionScript
  (bind _returnvalue (Transformation|GetActorLocation))
  (Rendering|Debug|FlushPersistentDebugLines)
  (Rendering|Debug|DrawDebugLine _returnvalue (+ _returnvalue (Math|Vector|MakeVector 0.0 0.0 (Variables|Default|GetjumpHeight))) "(R=0.843750,G=0.166764,B=0.183552,A=1.000000)" 9e+01 5.0))